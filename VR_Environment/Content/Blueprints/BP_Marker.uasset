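; BP_Marker is a marker actor, set up for VR, that draws on BP_Whiteboard surfaces.
; Each Tick it applies BrushColor to tip and body materials, then line traces a short distance along ArrowForward.
; A whiteboard hit calls OnPaintVisualLineTrace directly.
; Tick also chains RPC_Server to RPC_Client, which repeats the paint call using Tick's trace output rather than a passed parameter.
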(event `self.ReceiveTick`
  (params (DeltaSeconds :type "Float (single-precision)"))
  (bind _returnvalue (`KismetMathLibrary.Conv_LinearColorToVector` (`self.Brush Color`)))
  (`parent.ReceiveTick` DeltaSeconds)
  ;[1 0.6337 0.8576] Setting Color for body and tip
  (`MeshComponent.SetVectorParameterValueOnMaterials` (`self.Tip`) "Color" _returnvalue)
  (`MeshComponent.SetVectorParameterValueOnMaterials` (`self.Body`) "Color" _returnvalue)
  ;[1 0.1906 0.1906] VR Mode (If using marker, detect hit on target canvas)
  (if true
    (bind _hitresult (`self.DetectHitCanvasActor`))
    (`self.RPC_Server`)))

(event `RPC_Server`
  (`self.RPC_Client`))

(event `RPC_Client`
  (bind _asbp_whiteboard (cast `/Game/Blueprints/BP_Whiteboard` (`.HitActor` (`GameplayStatics.BreakHitResult` (stale `self.ReceiveTick` _hitresult)))))
  (`/Game/Blueprints/BP_Whiteboard.On Paint Visual Line Trace` _asbp_whiteboard self (stale `self.ReceiveTick` _hitresult)))

(fn `DetectHitCanvasActor`
  (returns (HitResult :type "HitResult Structure"))
  (bind _arrowforward (`self.ArrowForward`))
  (bind _returnvalue (`SceneComponent.K2_GetComponentLocation` _arrowforward))
  (bind (_outhit _returnvalue_2) (`KismetSystemLibrary.LineTraceSingleByProfile` :`Start` _returnvalue :`End` (+ _returnvalue (* (`KismetMathLibrary.GetForwardVector` (`SceneComponent.K2_GetComponentRotation` _arrowforward)) (`KismetMathLibrary.Conv_DoubleToVector` 15.0))) :`ProfileName` "BlockAllDynamic" :`bTraceComplex` true :`DrawDebugType` (`self.Draw Debug Type`)))
  ;[0.3552 0.3552 0.3552] Drawing on the Whiteboard
  (if _returnvalue_2
    (bind _asbp_whiteboard (cast `/Game/Blueprints/BP_Whiteboard` (`.HitActor` (`GameplayStatics.BreakHitResult` _outhit))))
    (`/Game/Blueprints/BP_Whiteboard.On Paint Visual Line Trace` _asbp_whiteboard self _outhit)
    (return _outhit)))

(fn `UserConstructionScript`)