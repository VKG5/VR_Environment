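; Whiteboard actor that displays brush strokes painted onto its mesh by a marker.
; On BeginPlay it creates a render target, binds it to the board's dynamic material as the BrushStroke texture, and creates a paint brush material instance.
; OnPaintVisualLineTrace converts the trace hit to a collision UV, passes it with the marker's size, color and strength to the brush material, and draws that material into the render target.
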(event `self.ReceiveBeginPlay`
  ;[1 0 0] May need to change the Element Index!!
  (bind _returnvalue (`PrimitiveComponent.CreateDynamicMaterialInstance` (`self.SM_Whiteboard`) 0 "/Game/Blueprints/Whiteboard/MI_Whiteboard.MI_Whiteboard" "None"))
  ;[0.2971 0.4094 1] Create Render Target and assign to texture - BrushTexture
  (bind _returnvalue_2 (`KismetRenderingLibrary.CreateRenderTarget2D` (`self.RenderTextureSizeX`) (`self.RenderTextureSizeY`)))
  (set `self.RenderToTexture` _returnvalue_2)
  (`MaterialInstanceDynamic.SetTextureParameterValue` _returnvalue "BrushStroke" _returnvalue_2)
  ;[1 0.1567 0.3516] Brush material instance creation
  (bind _returnvalue_3 (`KismetMaterialLibrary.CreateDynamicMaterialInstance` "/Game/Blueprints/Marker/MI_PaintMarker.MI_PaintMarker"))
  (set `self.BrushMaterialInstance` _returnvalue_3))

(fn `On Paint Visual Line Trace`
  (params (Marker :type "/Game/Blueprints/BP_Marker Object Reference") (`Hit Result` :type "HitResult Structure"))
  (bind (_x _y) (`KismetMathLibrary.BreakVector2D` (`GameplayStatics.FindCollisionUV` `Hit Result`)))
  (set `self.Brush` Marker)
  ;[0.4927 0.249 1] UV Coords from Hit and setting on Material Instance
  (`MaterialInstanceDynamic.SetVectorParameterValue` (`self.BrushMaterialInstance`) "HitPosition" (make `LinearColor` _x _y 0.0 1.0))
  ;[1 0.4732 0.09896] Set the Brush Size for the Material Instance
  (`MaterialInstanceDynamic.SetScalarParameterValue` (`self.BrushMaterialInstance`) "BrushSize" (`/Game/Blueprints/BP_Marker.Brush Size` (`self.Brush`)))
  ;[0.08608 0.6719 0.6122] Set Brush Color in Material Instance
  (`MaterialInstanceDynamic.SetVectorParameterValue` (`self.BrushMaterialInstance`) "BrushColor" (`/Game/Blueprints/BP_Marker.Brush Color` (`self.Brush`)))
  ;[0.3893 0.4771 1] Set Brush Strength in Material Instance
  (`MaterialInstanceDynamic.SetScalarParameterValue` (`self.BrushMaterialInstance`) "BrushStrength" (`/Game/Blueprints/BP_Marker.Brush Strength` (`self.Brush`)))
  ;[0 0 0] Draw material on Render Target
  (`KismetRenderingLibrary.DrawMaterialToRenderTarget` (`self.RenderToTexture`) (`self.BrushMaterialInstance`)))

(fn `UserConstructionScript`)